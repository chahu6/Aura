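; BP_Aura_MainMenu is the main menu scene actor for Aura, running the menu UI and its animated backdrop.
; BeginPlay plays the menu music, adds WBP_MainMenu to the viewport, and switches the player to UI-only input with a visible cursor.
; Tick bobs the FireBall on a wrapped sine wave around its starting location and spins the magic circle decal at a configurable rate.
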(event EventTick
  (params (DeltaSeconds :type Float%20%28single-precision%29))
  (CallFunction|UpdateTime DeltaSeconds)
  (Transformation|SetWorldLocation (Variables|Default|GetFireBall) (+ (Variables|Default|GetInitLocation) (Math|Vector|MakeVector 0.0 0.0 (CallFunction|SinTime))) false false)
  (Transformation|AddLocalRotation (Variables|Default|GetDecal) (Math|Rotator|MakeRotator (* (Utilities|Time|GetWorldDeltaSeconds) (Variables|Default|GetMagicCircleRotationRate)) 0.0 0.0) false false))

(event EventBeginPlay
  (bind _returnvalue (Game|GetPlayerController 0))
  (Variables|Default|SetInitLocation (Transformation|GetWorldLocation (Variables|Default|GetFireBall)))
  (Audio|PlaySound2D "/Game/Assets/Sounds/Music/Music_MainMenu.Music_MainMenu" 1.0 1.0 0.0 0 0)
  (bind _returnvalue_2 (UserInterface|CreateWidget "/Game/Blueprints/UI/MainMenu/WBP_MainMenu.WBP_MainMenu_C"))
  (UserInterface|Viewport|AddtoViewport _returnvalue_2 0)
  (Input|SetInputModeUIOnly _returnvalue _returnvalue_2 "DoNotLock" false)
  (Variables|/Script/Engine.PlayerController|SetbShowMouseCursor _returnvalue true))

(fn ConstructionScript)

(fn UpdateTime
  (params (DeltaTime :type Float%20%28double-precision%29))
  (Variables|Default|SetTime (+ DeltaTime (Variables|Default|GetTime)))
  (if (> (Variables|Default|GetTime) 6.283185)
    (Variables|Default|SetTime 0.0)))

(fn SinTime
  (return (* (Math|Trig|Sin(Radians) (Variables|Default|GetTime)) (Variables|Default|GetAmplitude))))