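; Enemy gameplay ability that summons random minions at shuffled spawn locations while the Shaman summon montage plays.
; The Montage.Attack.1 gameplay event starts a delayed loop that spawns each minion slightly raised, with yaw along the direction from the summoner, a default controller and a ground Niagara effect.
; Each spawn raises the avatar's minion count through an interface message, and the minion's OnDestroyed binding lowers it again.
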(event Custom|OnDestroyed_Event
  (params (DestroyedActor :type Actor%20Object%20Reference))
  (Class|CombatInterface|IncremenetMinionCount(Message) (Ability|GetAvatarActorfromActorInfo) -1))

(event Ability|EventActivateAbility
  (bind _output_get (Variables|Default|SetSpawnLocations (Class|AuraSummonAbility|GetSpawnLocations)))
  (Utilities|Array|Shuffle _output_get)
  (|PlayMontageandWaitProxy "None" "/Game/Assets/Enemies/Shaman/Animations/AM_Shaman_Summon.AM_Shaman_Summon" 1.0 "None" true 1.0 0.0
    (:then
      (Ability|Tasks|WaitGameplayEvent "(TagName=\"Montage.Attack.1\")" 0
        (:EventReceived
          (if (< (Variables|Default|GetSpawnLocationsIndex) (Utilities|Array|Length (Variables|Default|GetSpawnLocations))) :!label _label
            (bind _returnvalue (Game|SpawnActorfromClass (Class|AuraSummonAbility|GetRandomMinionClass) (Math|Transform|MakeTransform (+ (Utilities|Array|Get(acopy) (Variables|Default|GetSpawnLocations) (Variables|Default|GetSpawnLocationsIndex)) "0.000000,0.000000,70.000000") (Math|Rotator|MakeRotator 0.0 0.0 (.Yaw (Math|Rotator|BreakRotator (Math|Rotator|FindLookatRotation (Transformation|GetActorLocation (Ability|GetAvatarActorfromActorInfo)) (Utilities|Array|Get(acopy) (Variables|Default|GetSpawnLocations) (Variables|Default|GetSpawnLocationsIndex)))))) "1.000000,1.000000,1.000000") "AlwaysSpawn" "MultiplyWithRoot" 0 0))
            (Game|AssignOnDestroyed _returnvalue (delegate Custom|OnDestroyed_Event))
            (Pawn|SpawnDefaultController _returnvalue)
            (Class|CombatInterface|IncremenetMinionCount(Message) (Ability|GetAvatarActorfromActorInfo) 1)
            (Niagara|SpawnSystematLocation "/Game/Assets/Effects/Combat/NS_GroundSummon.NS_GroundSummon" (Utilities|Array|Get(acopy) (Variables|Default|GetSpawnLocations) (Variables|Default|GetSpawnLocationsIndex)))
            (Math|Integer|IncrementInt (Variables|Default|GetSpawnLocationsIndex)
              (:%20%20
                (Utilities|FlowControl|Delay 0.2)
                (goto _label)))))))))